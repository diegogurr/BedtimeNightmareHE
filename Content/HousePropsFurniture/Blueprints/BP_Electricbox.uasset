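; BP_Electricbox is a usable fuse box that restores electricity in the house.
; On Use it sets the shared CanTurnOnLights flag on HE_GameInstance, playing a switch sound and printing a status message, or only reports that power is already on.
; Tick polls that flag every frame to rotate the main switch mesh between its on and off positions.
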(event EventBeginPlay
  (bind _ashe_game_instance (Utilities|Casting|CastToHE_GameInstance (Game|GetGameInstance)))
  (Variables|Default|SetGameInstanceREF _ashe_game_instance))

(event EventUse
  (params (HorrorEvent :type Boolean))
  (bind _gameinstanceref (Variables|Default|GetGameInstanceREF))
  (if (Variables|/Game/HorrorEngine/Blueprints/Player/HE_GameInstance.HE_GameInstance_C|GetCanTurnOnLights _gameinstanceref)
    (Audio|PlaySound2D "/Game/Assets/Sounds/interruttore_luce_off.interruttore_luce_off" 1.0 1.0 0.0 0 0)
    (Development|PrintString "You already have electricity!")
    (else
      (Variables|/Game/HorrorEngine/Blueprints/Player/HE_GameInstance.HE_GameInstance_C|SetCanTurnOnLights _gameinstanceref true)
      (Audio|PlaySound2D "/Game/Assets/Sounds/interruttore_luce_on.interruttore_luce_on" 1.0 1.0 0.0 0 0)
      (Development|PrintString "Electricity is back! "))))

(event EventTick
  (params (DeltaSeconds :type Float%20%28single-precision%29))
  (bind _electricbox_mainswitch (Variables|Default|GetElectricbox_mainswitch))
  (if (Variables|/Game/HorrorEngine/Blueprints/Player/HE_GameInstance.HE_GameInstance_C|GetCanTurnOnLights (Variables|Default|GetGameInstanceREF))
    (Transformation|SetRelativeRotation _electricbox_mainswitch "0, 0, 0" false false)
    (else
      (Transformation|SetRelativeRotation _electricbox_mainswitch "0.000000,0.000000,90.000000" false false))))

(fn ConstructionScript)