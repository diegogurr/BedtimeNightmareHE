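; BP_Lamp_wall is a placeable wall lamp prop with an on or off look configured in the construction script.
; LampOn switches the shade and body meshes between emissive-on and off material instances.
; The point light is kept only when LampOn and AddLight are both set, otherwise it is destroyed.
; When off, the shade is also set to static mobility; the event graph is unused.
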(event EventBeginPlay)

(event Collision|EventActorBeginOverlap
  (params (OtherActor :type Actor%20Object%20Reference)))

(event EventTick
  (params (DeltaSeconds :type Float%20%28single-precision%29)))

(fn ConstructionScript
  (if (Variables|Lamp|GetLamp%20On?)
    (Rendering|Material|SetMaterial (Variables|Default|GetLamp_wall_shade) 0 "/Game/HousePropsFurniture/Materials/MI_Lamps_B_on.MI_Lamps_B_on")
    (Rendering|Material|SetMaterial (Variables|Default|GetLamp_wall_body) 0 "/Game/HousePropsFurniture/Materials/MI_Lamps_B_on.MI_Lamps_B_on")
    (if (not (Variables|Lamp|GetAdd%20Light?))
      (Components|DestroyComponent (Variables|Default|GetPointLight)))
    (else
      (Components|DestroyComponent (Variables|Default|GetPointLight))
      (Rendering|Material|SetMaterial (Variables|Default|GetLamp_wall_shade) 0 "/Game/HousePropsFurniture/Materials/MI_Lamps_B_off.MI_Lamps_B_off")
      (Rendering|Material|SetMaterial (Variables|Default|GetLamp_wall_body) 0 "/Game/HousePropsFurniture/Materials/MI_Lamps_B_off.MI_Lamps_B_off")
      (Transformation|SetMobility (Variables|Default|GetLamp_wall_shade) "Static"))))