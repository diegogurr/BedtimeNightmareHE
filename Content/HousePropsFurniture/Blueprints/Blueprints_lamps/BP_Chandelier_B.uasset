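; Chandelier prop that switches on and off, swapping shade and body materials and toggling its point light.
; BeginPlay calls CloseOff, caches the game instance and light manager, and finds its BP_RoomZone with a small sphere trace at its location.
; Each state change notifies the light manager and room zone.
; The construction script previews the lamp state and removes the point light when off or when AddLight is false.
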(event EventBeginPlay
  (bind _returnvalue (Transformation|GetActorLocation))
  ;[0.4072 0.4072 0.4072] BeginPlay
  (CallFunction|Close/Off false)
  (bind _ashe_game_instance (Utilities|Casting|CastToHE_GameInstance (Game|GetGameInstance)))
  (Variables|Default|SetGameInstanceREF _ashe_game_instance)
  (bind _returnvalue_2 (Actor|GetActorOfClass "/Game/Blueprints/Lights/BP_LightManager.BP_LightManager_C"))
  (Variables|Default|SetLightManagerREF _returnvalue_2)
  (bind _outhit (Collision|SphereTraceForObjects _returnvalue _returnvalue 16.0 (Utilities|Array|MakeArray "ObjectTypeQuery8") false 0 "None"))
  (bind _asbp_room_zone (Utilities|Casting|CastToBP_RoomZone (.hitactor _outhit)))
  (Utilities|IsValid (Variables|RoomZone|GetRoomZoneREF)
    (:Is%20Not%20Valid
      (Variables|RoomZone|SetRoomZoneREF _asbp_room_zone))))

(event EventOpen/On
  (params (HorrorEvent :type Boolean))
  (bind _lightmanagerref (Variables|Default|GetLightManagerREF))
  (bind _roomzoneref (Variables|RoomZone|GetRoomZoneREF))
  ;[0.1683 0.1683 0.1683] On/Off Settings
  (if (not (Variables|Lamp|GetLamp%20On?))
    (Variables|Lamp|SetLamp%20On? true)
    (Rendering|Material|SetMaterial (Variables|Default|GetChandelier_B_shades) 0 "/Game/HousePropsFurniture/Materials/MI_Lamps_B_on.MI_Lamps_B_on")
    (Rendering|Material|SetMaterial (Variables|Default|GetChandelier_B_body) 0 "/Game/HousePropsFurniture/Materials/MI_Lamps_B_on.MI_Lamps_B_on")
    (Rendering|SetVisibility (Variables|Default|GetPointLight) true false)
    (Utilities|IsValid _lightmanagerref
      (:Is%20Valid
        (Default|UpdateLights _lightmanagerref (Variables|Lamp|GetLamp%20On?))
        (Utilities|IsValid _roomzoneref
          (:Is%20Valid
            (Default|UpdateLightStatus _roomzoneref (Variables|Lamp|GetLamp%20On?))))))))

(event EventClose/Off
  (params (HorrorEvent :type Boolean))
  (bind _lightmanagerref (Variables|Default|GetLightManagerREF))
  (bind _roomzoneref (Variables|RoomZone|GetRoomZoneREF))
  ;[0.1683 0.1683 0.1683] On/Off Settings
  (if (Variables|Lamp|GetLamp%20On?)
    (Variables|Lamp|SetLamp%20On? false)
    (Rendering|Material|SetMaterial (Variables|Default|GetChandelier_B_shades) 0 "/Game/HousePropsFurniture/Materials/MI_Lamps_B_off.MI_Lamps_B_off")
    (Rendering|Material|SetMaterial (Variables|Default|GetChandelier_B_body) 0 "/Game/HousePropsFurniture/Materials/MI_Lamps_B_off.MI_Lamps_B_off")
    (Rendering|SetVisibility (Variables|Default|GetPointLight) false false)
    (Utilities|IsValid _lightmanagerref
      (:Is%20Valid
        (Default|UpdateLights _lightmanagerref (Variables|Lamp|GetLamp%20On?))
        (Utilities|IsValid _roomzoneref
          (:Is%20Valid
            (Default|UpdateLightStatus _roomzoneref (Variables|Lamp|GetLamp%20On?))))))))

(fn ConstructionScript
  (if (Variables|Lamp|GetLamp%20On?)
    (Rendering|Material|SetMaterial (Variables|Default|GetChandelier_B_shades) 0 "/Game/HousePropsFurniture/Materials/MI_Lamps_B_on.MI_Lamps_B_on")
    (Rendering|Material|SetMaterial (Variables|Default|GetChandelier_B_body) 0 "/Game/HousePropsFurniture/Materials/MI_Lamps_B_on.MI_Lamps_B_on")
    (if (not (Variables|Lamp|GetAdd%20Light?))
      (Components|DestroyComponent (Variables|Default|GetPointLight)))
    (else
      (Components|DestroyComponent (Variables|Default|GetPointLight))
      (Rendering|Material|SetMaterial (Variables|Default|GetChandelier_B_shades) 0 "/Game/HousePropsFurniture/Materials/MI_Lamps_B_off.MI_Lamps_B_off")
      (Rendering|Material|SetMaterial (Variables|Default|GetChandelier_B_body) 0 "/Game/HousePropsFurniture/Materials/MI_Lamps_B_off.MI_Lamps_B_off")
      (Transformation|SetMobility (Variables|Default|GetChandelier_B_shades) "Static"))))