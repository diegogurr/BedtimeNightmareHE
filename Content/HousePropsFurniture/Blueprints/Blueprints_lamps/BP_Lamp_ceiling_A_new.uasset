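; Switchable ceiling lamp that toggles its emissive-style on/off material and point light, with a turn-off hook for blackouts.
; On BeginPlay it switches off, caches the game instance and light manager, and finds its room zone with a small sphere trace.
; State changes report to the light manager and room zone.
; The construction script previews the material and removes the point light when the lamp starts off or AddLight is false.
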(event EventTurnOffFunction
  ;[0.15 0.15 0.15 0.5] Blackout
  (CallFunction|Close/Off false))

(event EventBeginPlay
  (bind _returnvalue (Transformation|GetActorLocation))
  ;[0.4072 0.4072 0.4072] BeginPlay
  (CallFunction|Close/Off false)
  (bind _ashe_game_instance (Utilities|Casting|CastToHE_GameInstance (Game|GetGameInstance)))
  (Variables|Default|SetGameInstanceREF _ashe_game_instance)
  (bind _returnvalue_2 (Actor|GetActorOfClass "/Game/Blueprints/Lights/BP_LightManager.BP_LightManager_C"))
  (Variables|Default|SetLightManagerREF _returnvalue_2)
  (bind _outhit (Collision|SphereTraceForObjects _returnvalue _returnvalue 16.0 (Utilities|Array|MakeArray "ObjectTypeQuery8") false 0 "None"))
  (bind _asbp_room_zone (Utilities|Casting|CastToBP_RoomZone (.hitactor _outhit)))
  (Utilities|IsValid (Variables|RoomZone|GetRoomZoneREF)
    (:Is%20Not%20Valid
      (Variables|RoomZone|SetRoomZoneREF _asbp_room_zone))))

(event EventClose/Off
  (params (HorrorEvent :type Boolean))
  (bind _lightmanagerref (Variables|Default|GetLightManagerREF))
  (bind _roomzoneref (Variables|RoomZone|GetRoomZoneREF))
  ;[0.1683 0.1683 0.1683] On/Off Settings
  (if (Variables|Default|GetLamp%20On?)
    (Variables|Default|SetLamp%20On? false)
    (Rendering|Material|SetMaterial (Variables|Default|GetStaticMesh) 0 "/Game/HousePropsFurniture/Materials/MI_Lamps_C_OFF.MI_Lamps_C_off")
    (Rendering|SetVisibility (Variables|Default|GetPointLight) false false)
    (Utilities|IsValid _lightmanagerref
      (:Is%20Valid
        (Default|UpdateLights _lightmanagerref (Variables|Default|GetLamp%20On?) 1.0)
        (Utilities|IsValid _roomzoneref
          (:Is%20Valid
            (Default|UpdateLightStatus _roomzoneref (Variables|Default|GetLamp%20On?))))))))

(event EventOpen/On
  (params (HorrorEvent :type Boolean))
  (bind _lightmanagerref (Variables|Default|GetLightManagerREF))
  (bind _roomzoneref (Variables|RoomZone|GetRoomZoneREF))
  ;[0.1683 0.1683 0.1683] On/Off Settings
  (if (not (Variables|Default|GetLamp%20On?))
    (Variables|Default|SetLamp%20On? true)
    (Rendering|Material|SetMaterial (Variables|Default|GetStaticMesh) 0 "/Game/HousePropsFurniture/Materials/MI_Lamps_C_on.MI_Lamps_C_on")
    (Rendering|SetVisibility (Variables|Default|GetPointLight) true false)
    (Utilities|IsValid _lightmanagerref
      (:Is%20Valid
        (Default|UpdateLights _lightmanagerref (Variables|Default|GetLamp%20On?) 1.0)
        (Utilities|IsValid _roomzoneref
          (:Is%20Valid
            (Default|UpdateLightStatus _roomzoneref (Variables|Default|GetLamp%20On?))))))))

(fn ConstructionScript
  (if (Variables|Default|GetLamp%20On?)
    (Rendering|Material|SetMaterial (Variables|Default|GetStaticMesh) 0 "/Game/HousePropsFurniture/Materials/MI_Lamps_C_on.MI_Lamps_C_on")
    (if (not (Variables|Default|GetAdd%20Light?))
      (Components|DestroyComponent (Variables|Default|GetPointLight)))
    (else
      (Components|DestroyComponent (Variables|Default|GetPointLight))
      (Rendering|Material|SetMaterial (Variables|Default|GetStaticMesh) 0 "/Game/HousePropsFurniture/Materials/MI_Lamps_C_OFF.MI_Lamps_C_off"))))