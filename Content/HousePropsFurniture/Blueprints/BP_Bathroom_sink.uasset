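; BP_Bathroom_sink is a bathroom sink that acts as a hold-to-complete task.
; UseHeld starts a looping CheckHoldTime timer and shows a progress bar widget, which ReleaseHeld cancels and removes.
; CheckHoldTime fills the bar from elapsed time against HoldTime.
; On completion it notifies the game instance's task manager with ItemID, removes the bar and sets IsCompleted.
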(event EventUseHeld
  (params (HorrorEvent :type Boolean))
  (Variables|Default|GetIs%20Completed
    (:then)
    (:else
      (Variables|Default|SetHoldStartTime (Utilities|Time|GetGameTimeinSeconds))
      (Utilities|Time|SetTimerbyFunctionName 0 "CheckHoldTime" 0.2 true)
      (bind _returnvalue (UserInterface|CreateWidget "/Game/Blueprints/UI/WBP_TaskProgressBar.WBP_TaskProgressBar_C"))
      (bind _output_get (Variables|Default|SetProgressBarREF _returnvalue))
      (UserInterface|Viewport|AddtoViewport _output_get 0))))

(event EventReleaseHeld
  (params (HorrorEvent :type Boolean))
  (Variables|Default|GetIs%20Completed
    (:then)
    (:else
      (Variables|Default|SetHoldStartTime 0.0)
      (Utilities|Time|ClearTimerbyFunctionName 0 "CheckHoldTime")
      (Development|PrintString "Task interrupted!")
      (Widget|RemovefromParent (Variables|Default|GetProgressBarREF)))))

(fn ConstructionScript)

(fn CheckHoldTime
  (bind _returnvalue (Utilities|Time|GetGameTimeinSeconds))
  (bind _holdstarttime (Variables|Default|GetHoldStartTime))
  (bind _returnvalue_2 (- _returnvalue _holdstarttime))
  (Progress|SetPercent (Variables|/Game/Blueprints/UI/WBP_TaskProgressBar.WBP_TaskProgressBar_C|GetTaskProgressBar (Variables|Default|GetProgressBarREF)) (/ _returnvalue_2 (Variables|Default|GetHoldTime)))
  (if (>= _returnvalue_2 (Variables|Default|GetHoldTime))
    (bind _ashe_game_instance (Utilities|Casting|CastToHE_GameInstance (Game|GetGameInstance)))
    (Default|NotifyTaskfromWorld (Variables|/Game/HorrorEngine/Blueprints/Player/HE_GameInstance.HE_GameInstance_C|GetTaskManagerRef _ashe_game_instance) (Variables|Default|GetItemID))
    (Utilities|Time|ClearTimerbyFunctionName 0 "CheckHoldTime")
    (Development|PrintString "Press task completed!")
    (Widget|RemovefromParent (Variables|Default|GetProgressBarREF))
    (Variables|Default|SetIs%20Completed true)))