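; Spawn manager that randomly places a set of relocatable objects at registered spawn points when play begins.
; Spawn points add themselves or are added through RegisterSpawnPoint.
; After a one-second delay on BeginPlay, it shuffles both lists and snap-attaches each object to a point's BP_SpawnPoint component, matching location and rotation.
; Each used point leaves the list, so none repeats; there is no check for running out.
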(event EventBeginPlay
  (bind _actorstorelocate (Variables|Default|GetActorsToRelocate))
  (Utilities|FlowControl|Delay 1.0)
  (Utilities|Array|Shuffle (Variables|Default|GetSpawnPoints))
  (Utilities|Array|Shuffle _actorstorelocate)
  (for _array_element _actorstorelocate
    (Transformation|AttachComponentToComponent _array_element (Actor|GetComponentbyClass (Utilities|Array|Get(acopy) (Variables|Default|GetSpawnPoints)) "/Game/Blueprints/BP_SpawnPoint.BP_SpawnPoint_C") "None" "SnapToTarget" "SnapToTarget" "KeepRelative" true)
    (Utilities|Array|RemoveIndex (Variables|Default|GetSpawnPoints))))

(fn ConstructionScript)

(fn RegisterSpawnPoint
  (params (SpawnPointRef :type Actor%20Object%20Reference))
  (Utilities|Array|Add (Variables|Default|GetSpawnPoints) SpawnPointRef))