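; BP_LightManager manages a shared light battery that drains under lighting load and causes blackouts when empty.
; UpdateLights tracks total voltage; Tick drains the battery by that load or recharges it at zero load, mirroring the level to HE_GameInstance.
; TriggerBlackout disables lights via BPI_LightInteractable and clears CanTurnOnLights, pausing battery updates until that flag is restored externally.
; Post-blackout recharge uses the generator speed multiplier.
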(event EventTick
  (params (DeltaSeconds :type Float%20%28single-precision%29))
  (bind _batteryincrement (Variables|Default|GetBatteryIncrement))
  (if (Variables|/Game/HorrorEngine/Blueprints/Player/HE_GameInstance.HE_GameInstance_C|GetCanTurnOnLights (Variables|Default|GetGameInstanceRef))
    (if (> (Variables|Default|GetLightsVoltage) 0.0)
      (bind _output_get (Variables|Default|SetBatteryCurrent (Math|Float|Clamp(Float) (- (Variables|Default|GetBatteryCurrent) (* (Variables|Default|GetBatteryDecrement) (Variables|Default|GetLightsVoltage))) 0.0 (Variables|Default|GetBatteryMax))))
      (Variables|/Game/HorrorEngine/Blueprints/Player/HE_GameInstance.HE_GameInstance_C|SetCurrentBatteryLevel (Variables|Default|GetGameInstanceRef) (Variables|Default|GetBatteryCurrent))
      (if (<= _output_get 0.0)
        (CallFunction|TriggerBlackout))
      (else
        (Variables|Default|SetBatteryCurrent (Math|Float|Clamp(Float) (+ (Variables|Default|GetBatteryCurrent) (Math|Float|SelectFloat (* _batteryincrement (Variables|Default|GetGeneratorRechargeSpeed)) _batteryincrement (Variables|Default|GetBlackoutTriggered))) 0.0 (Variables|Default|GetBatteryMax)))
        (Variables|/Game/HorrorEngine/Blueprints/Player/HE_GameInstance.HE_GameInstance_C|SetCurrentBatteryLevel (Variables|Default|GetGameInstanceRef) (Variables|Default|GetBatteryCurrent))
        (if (>= (Variables|Default|GetBatteryCurrent) (Variables|Default|GetBatteryMax))
          (Variables|Default|SetBlackoutTriggered false))))))

(event EventBeginPlay
  (bind _batterymax (Variables|Default|GetBatteryMax))
  (bind _ashe_game_instance (Utilities|Casting|CastToHE_GameInstance (Game|GetGameInstance)))
  (bind _output_get (Variables|Default|SetGameInstanceRef _ashe_game_instance))
  (Variables|/Game/HorrorEngine/Blueprints/Player/HE_GameInstance.HE_GameInstance_C|SetCurrentBatteryLevel _output_get _batterymax)
  (Variables|/Game/HorrorEngine/Blueprints/Player/HE_GameInstance.HE_GameInstance_C|SetCanTurnOnLights _output_get true)
  (Variables|Default|SetBatteryCurrent _batterymax))

(fn ConstructionScript)

(fn UpdateLights
  (params (LightTurnedOn :type Boolean) (LightVoltage :type Float%20%28double-precision%29))
  (if LightTurnedOn
    (Variables|Default|SetLightsVoltage (+ (Variables|Default|GetLightsVoltage) LightVoltage))
    (Variables|Default|SetBlackoutTriggered false)
    (else
      (Variables|Default|SetLightsVoltage (Math|Float|Clamp(Float) (- (Variables|Default|GetLightsVoltage) LightVoltage) 0.0 1e+02))))
  (Development|PrintString (Utilities|String|Append "Lights On:" (Utilities|String|ToString(Float) (Variables|Default|GetLightsVoltage))))
  (return))

(fn TriggerBlackout
  (Development|PrintString "BLACKOUT!" true true "(R=1.000000,G=0.011735,B=0.000000,A=1.000000)" 4.0)
  (Variables|/Game/HorrorEngine/Blueprints/Player/HE_GameInstance.HE_GameInstance_C|SetCanTurnOnLights (Variables|Default|GetGameInstanceRef) false)
  (for _array_element (Variables|Default|GetLightReferences)
    (if (Utilities|DoesObjectImplementInterface _array_element "/Game/Blueprints/BPI_LightInteractable.BPI_LightInteractable_C")
      (Class|BPILightInteractable|TurnOffFunction(Message) _array_element)
      (Variables|Default|SetLightsVoltage 0.0)
      (Audio|PlaySound2D "/Game/Assets/Audio/AC_CuttingPower_Cue.AC_CuttingPower_Cue" 1.0 1.0 0.0 0 0)
      (Variables|Default|SetBlackoutTriggered true))))