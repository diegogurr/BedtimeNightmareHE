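; BP_Monster is an AI-controlled monster that can relocate among spawn points and toggle collision on its attached actors.
; On BeginPlay it caches its AI controller, writes its starting location to the blackboard as home, and gathers all BP_MonsterSpawnPoint actors.
; Despite its name, TeleportToRandomLocation makes a swept move to the first spawn point at or beyond a threshold distance from the player.
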(event EventBeginPlay
  (bind _asbp_monster_aicontroller (Utilities|Casting|CastToBP_MonsterAIController (Pawn|GetController)))
  (Variables|Default|SetBPMonsterAIControllerRef _asbp_monster_aicontroller)
  (bind _output_get (Variables|Default|SetHomeLocation (Transformation|GetActorLocation)))
  (AI|Components|Blackboard|SetValueasVector (AI|GetBlackboard 0) (Variables|Default|GetHomeLocationName) _output_get)
  (bind _outactors (Actor|GetAllActorsOfClass "/Game/BedtimeNightmare/Blueprints/AI/BP_MonsterSpawnPoint.BP_MonsterSpawnPoint_C"))
  (Variables|Default|SetSpawnPoints _outactors))

(fn ConstructionScript)

(fn TeleporttoRandomLocation
  (Utilities|FlowControl|DoOnce false
    (:Completed
      (bind _array_element (Utilities|Array|ForEachLoopwithBreak (Variables|Default|GetSpawnPoints))
        (:LoopBody
          (if (>= (Transformation|GetDistanceTo (Game|GetPlayerCharacter 0) _array_element) (LocalVariables|GetDistanceTreshold))
            (Transformation|SetActorLocation (Transformation|GetActorLocation _array_element) true false)
            (return)))
        (:Completed
          (return))))))

(fn EnableChildren
  (for _array_element (Actor|GetAttachedActors true false)
    (Collision|SetActorEnableCollision _array_element true)))

(fn DisableChildren
  (for _array_element (Actor|GetAttachedActors true false)
    (Collision|SetActorEnableCollision _array_element false)))