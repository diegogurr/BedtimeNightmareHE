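; BP_RoomZone is a box-shaped volume that tracks room lighting for actors implementing BPI_LightReceiver.
; The construction script sizes the box from BoxDimensions.
; When such an actor begins or ends overlap, the zone adds or removes itself on HE_GameInstance, then triggers UpdateRoomLights.
; UpdateLightStatus stores the zone's IsLit state and asks the game instance to refresh room lights.
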(event OnComponentBeginOverlap(BoxCollision)
  (params (OverlappedComponent :type Primitive%20Component%20Object%20Reference) (OtherActor :type Actor%20Object%20Reference) (OtherComp :type Primitive%20Component%20Object%20Reference) (OtherBodyIndex :type Integer) (bFromSweep :type Boolean) (SweepResult :type Hit%20Result%20Structure%20%28by%20ref%29))
  (if (Utilities|DoesObjectImplementInterface OtherActor "/Game/BedtimeNightmare/Blueprints/Lights/BPI_LightReceiver.BPI_LightReceiver_C")
    (CallFunction|AddRoomZone)))

(event OnComponentEndOverlap(BoxCollision)
  (params (OverlappedComponent :type Primitive%20Component%20Object%20Reference) (OtherActor :type Actor%20Object%20Reference) (OtherComp :type Primitive%20Component%20Object%20Reference) (OtherBodyIndex :type Integer))
  (if (Utilities|DoesObjectImplementInterface OtherActor "/Game/BedtimeNightmare/Blueprints/Lights/BPI_LightReceiver.BPI_LightReceiver_C")
    (CallFunction|RemoveRoomZone)))

(event EventBeginPlay
  (bind _ashe_game_instance (Utilities|Casting|CastToHE_GameInstance (Game|GetGameInstance)))
  (Variables|Default|SetGameInstanceREF _ashe_game_instance))

(fn ConstructionScript
  (Components|Box|SetBoxExtent (Variables|Default|GetBoxCollision) (Variables|Default|GetBox%20Dimensions) true))

(fn UpdateLightStatus
  (params (IsOn :type Boolean))
  (Variables|Default|SetIsLit IsOn)
  (Default|UpdateRoomLights (Variables|Default|GetGameInstanceREF)))

(fn AddRoomZone
  (bind _gameinstanceref (Variables|Default|GetGameInstanceREF))
  (Default|AddRoomZone _gameinstanceref self)
  (Default|UpdateRoomLights _gameinstanceref))

(fn RemoveRoomZone
  (bind _gameinstanceref (Variables|Default|GetGameInstanceREF))
  (Default|RemoveRoomZone _gameinstanceref self)
  (Default|UpdateRoomLights _gameinstanceref))