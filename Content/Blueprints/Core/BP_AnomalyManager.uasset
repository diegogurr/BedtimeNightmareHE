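; Anomaly manager that activates random anomalies from its Anomalies list at randomized intervals during play.
; BeginPlay disables collision on every anomaly and starts a named timer for ActivateRandomAnomaly, using actor collision as the active flag.
; That function gathers collision-disabled anomalies into HiddenAnomalies, enables collision on a random entry, then re-arms the timer with extra random jitter.
; Debug messages report each activation, or an empty pool, which skips rescheduling.
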(event EventBeginPlay
  (for _array_element (Variables|AnomaliesSettings|GetAnomalies)
    (Collision|SetActorEnableCollision _array_element false)
    (Utilities|Time|SetTimerbyFunctionName 0 "ActivateRandomAnomaly" (Math|Random|RandomFloatinRange (Variables|AnomaliesSettings|GetActivationMinInterval) (Variables|AnomaliesSettings|GetActivationMaxInterval)))))

(fn ConstructionScript)

(fn ActivateRandomAnomaly
  (bind _hiddenanomalies (LocalVariables|GetHiddenAnomalies))
  (bind _hiddenanomalies_2 (LocalVariables|GetHiddenAnomalies))
  (for _array_element (Variables|AnomaliesSettings|GetAnomalies)
    (if (not (Collision|GetActorEnableCollision _array_element))
      (Utilities|Array|Add _hiddenanomalies _array_element)))
  (if (== (Utilities|Array|Length _hiddenanomalies) 0)
    (Development|PrintString "Nessuna anomalia!" true true "(R=0.963496,G=1.000000,B=0.000000,A=1.000000)")
    (else
      (Collision|SetActorEnableCollision (Utilities|Array|Get(acopy) _hiddenanomalies_2 (Math|Random|RandomIntegerinRange 0 (- (Utilities|Array|Length _hiddenanomalies_2) 1))) true)
      (Development|PrintString "ANOMALIA!" true true "(R=0.963496,G=1.000000,B=0.000000,A=1.000000)")
      (Utilities|Time|SetTimerbyFunctionName 0 "ActivateRandomAnomaly" (+ (Math|Random|RandomFloatinRange (Variables|AnomaliesSettings|GetActivationMinInterval) (Variables|AnomaliesSettings|GetActivationMaxInterval)) (Math|Random|RandomFloatinRange -1e+01 1e+01))))))