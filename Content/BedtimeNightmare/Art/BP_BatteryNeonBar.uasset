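; BP_BatteryNeonBar is a neon bar actor that visually displays the remaining battery tracked by the light manager.
; On BeginPlay it creates a dynamic instance of M_NeonFillBar on its static mesh and caches the first BP_LightManager found in the level.
; Every tick it divides the manager's current battery by its maximum and writes the ratio to the material's Fill parameter.
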(event EventBeginPlay
  (bind _returnvalue (Rendering|Material|CreateDynamicMaterialInstance (Variables|Debug|GetStaticMeshComponent) 0 "/Game/BedtimeNightmare/Materials/M_NeonFillBar.M_NeonFillBar" "None" :!class /Script/Engine.PrimitiveComponent))
  (Variables|Default|SetMID_Bar _returnvalue)
  (bind _outactors (Actor|GetAllActorsOfClass "/Game/BedtimeNightmare/Blueprints/Lights/BP_LightManager.BP_LightManager_C"))
  (Variables|Default|SetLightManagerRef (Utilities|Array|Get(acopy) _outactors)))

(event Collision|EventActorBeginOverlap
  (params (OtherActor :type Actor%20Object%20Reference)))

(event EventTick
  (params (DeltaSeconds :type Float%20%28single-precision%29))
  (bind _lightmanagerref (Variables|Default|GetLightManagerRef))
  (bind _output_get (Variables|Default|SetBattery01 (/ (Variables|/Game/BedtimeNightmare/Blueprints/Lights/BP_LightManager.BP_LightManager_C|GetBatteryCurrent _lightmanagerref) (Variables|/Game/BedtimeNightmare/Blueprints/Lights/BP_LightManager.BP_LightManager_C|GetBatteryMax _lightmanagerref))))
  (Rendering|Material|SetScalarParameterValue (Variables|Default|GetMID_Bar) "Fill" _output_get :!class /Script/Engine.MaterialInstanceDynamic))

(fn ConstructionScript)