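; BP_Doll is an anomaly doll that hides when the player looks toward it and shows only when off the center of view.
; Each Tick it takes the dot product of the player camera's forward vector and the normalized direction from camera to mesh.
; The mesh is visible while that value is at or below MaxVisibleRange, with no occlusion or distance check.
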(event EventBeginPlay)

(event Collision|EventActorBeginOverlap
  (params (OtherActor :type Actor%20Object%20Reference)))

(event EventTick
  (params (DeltaSeconds :type Float%20%28single-precision%29))
  (bind _returnvalue (Game|GetPlayerCameraManager 0))
  (Rendering|SetVisibility (Variables|Debug|GetStaticMeshComponent) (<= (Math|Vector|DotProduct (Math|Vector|GetForwardVector (Variables|/Script/Engine.PlayerCameraManager|GetTransformComponent _returnvalue)) (Math|Vector|Normalize (- (Transformation|GetWorldLocation (Variables|Debug|GetStaticMeshComponent)) (Transformation|GetWorldLocation (Variables|/Script/Engine.PlayerCameraManager|GetTransformComponent _returnvalue))))) (Variables|Default|GetMaxVisibleRange)) false))

(fn ConstructionScript)