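; BP_Collectible is a pickup that unlocks its CollectibleType in HE_GameInstance when it receives AlternativeUse.
; On BeginPlay it asks the game instance whether that type is already owned, and shows its skeletal mesh and activates its audio only if not.
; AlternativeUse hides the mesh, deactivates the audio, plays a 2D pickup cue and records the unlock, without destroying the actor.
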(event EventBeginPlay
  (bind _ashe_game_instance (Utilities|Casting|CastToHE_GameInstance (Game|GetGameInstance)))
  (bind _output_get (Variables|Default|SetAs%20HE%20Game%20Instance _ashe_game_instance))
  (bind _collectibleunlocked (Default|HasCollectible _output_get (Variables|Default|GetCollectibleType)))
  (Rendering|SetVisibility (Variables|Default|GetSkeletalMesh) (not _collectibleunlocked) false)
  (Components|Activation|SetActive (Variables|Default|GetCollectibleAudio) (not _collectibleunlocked) false))

(event EventAlternativeUse
  (params (HorrorEvent :type Boolean))
  (Rendering|SetVisibility (Variables|Default|GetSkeletalMesh) false false)
  (Components|Activation|SetActive (Variables|Default|GetCollectibleAudio) false false)
  (Audio|PlaySound2D "/Game/BedtimeNightmare/Audio/AC_Collectible_Cue.AC_Collectible_Cue" 0.4 1.0 0.0 0 0)
  (Default|UnlockCollectible (Variables|Default|GetAs%20HE%20Game%20Instance) (Variables|Default|GetCollectibleType)))

(fn ConstructionScript)