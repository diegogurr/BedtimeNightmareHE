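; Monster enemy that jumpscares the player on contact, unlocks an ending and opens the game over level.
; On BeginPlay it caches its AI controller, stores its home location in the Blackboard and gathers all monster spawn points.
; The jumpscare switches the camera to the monster with sound, spotlight and a random animation.
; Helpers toggle attached-actor collision and, once only, move it to the first sufficiently distant spawn point, despite the function's "random" name.
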(event OnComponentBeginOverlap(PlayerDetectionBox)
  (params (OverlappedComponent :type Primitive%20Component%20Object%20Reference) (OtherActor :type Actor%20Object%20Reference) (OtherComp :type Primitive%20Component%20Object%20Reference) (OtherBodyIndex :type Integer) (bFromSweep :type Boolean) (SweepResult :type Hit%20Result%20Structure%20%28by%20ref%29))
  (if (== OtherActor (Game|GetPlayerCharacter 0))
    (CallFunction|Jumpscare)))

(event Custom|Jumpscare
  (Components|Activation|SetActive (Variables|Default|GetChaseAudio) false false)
  (Collision|SetCollisionEnabled (Variables|Default|GetPlayer%20Detection%20Box) "NoCollision")
  (Audio|PlaySound2D "/Game/BedtimeNightmare/Audio/AC_Jumpscare_Cue.AC_Jumpscare_Cue" 1.0 1.0 0.0 0 0)
  (Rendering|SetVisibility (Variables|Default|GetSpotLight) true false)
  (Game|Player|SetViewTargetwithBlend (Game|GetPlayerController 0) self 0.0 "VTBlend_Linear" 0.0 false)
  (Components|Animation|PlayAnimation (Variables|Character|GetMesh) (Utilities|Select :Index (Math|Random|RandomIntegerinRange 0 1) :Option%200 "/Game/ThirdParty/Creepy_Mannequin/Demo/Zombie_Attack.Zombie_Attack" :Option%201 "/Game/ThirdParty/Creepy_Mannequin/Demo/Zombie_Scream.Zombie_Scream") false)
  (Input|DisableInput (Game|GetPlayerController 0))
  (bind _ashe_game_instance (Utilities|Casting|CastToHE_GameInstance (Game|GetGameInstance)))
  (Default|UnlockEnding _ashe_game_instance "NewEnumerator0")
  (Utilities|FlowControl|Delay 2.0)
  (Game|OpenLevel(byObjectReference) "/Game/BedtimeNightmare/Maps/L_GameOver.L_GameOver"))

(event EventBeginPlay
  (bind _asbp_monster_aicontroller (Utilities|Casting|CastToBP_MonsterAIController (Pawn|GetController)))
  (Variables|Default|SetBPMonsterAIControllerRef _asbp_monster_aicontroller)
  (bind _output_get (Variables|Default|SetHomeLocation (Transformation|GetActorLocation)))
  (AI|Components|Blackboard|SetValueasVector (AI|GetBlackboard 0) (Variables|Default|GetHomeLocationName) _output_get)
  (bind _outactors (Actor|GetAllActorsOfClass "/Game/BedtimeNightmare/Blueprints/AI/BP_MonsterSpawnPoint.BP_MonsterSpawnPoint_C"))
  (Variables|Default|SetSpawnPoints _outactors))

(fn ConstructionScript)

(fn TeleporttoRandomLocation
  (Utilities|FlowControl|DoOnce false
    (:Completed
      (for _array_element (Variables|Default|GetSpawnPoints)
        (if (>= (Transformation|GetDistanceTo (Game|GetPlayerCharacter 0) _array_element) (LocalVariables|GetDistanceTreshold))
          (Transformation|SetActorLocation (Transformation|GetActorLocation _array_element) true false)
          (return))))))

(fn EnableChildren
  (for _array_element (Actor|GetAttachedActors true false)
    (Collision|SetActorEnableCollision _array_element true)))

(fn DisableChildren
  (for _array_element (Actor|GetAttachedActors true false)
    (Collision|SetActorEnableCollision _array_element false)))