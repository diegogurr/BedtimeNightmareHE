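; Light manager for Bedtime Nightmare that runs the battery powering the lights and mirrors its level to the game instance.
; Lights report voltage through UpdateLights; Tick drains the battery by total voltage, with a lower multiplier as more lights are on, or recharges it at zero voltage.
; Near-empty charge triggers a blackout, shutting off referenced lights and the electric box.
; Battery updates then pause until IncreaseBatteryLevel re-enables lights; game completion also stops them.
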(event Custom|OnGameCompleted_Received
  (Variables|Default|SetbIsGameCompleted true))

(event Custom|Increase%20Battery%20Level
  (params (Increase%20Value :type Float%20%28double-precision%29))
  (Variables|Default|SetBatteryCurrent (Math|Float|Clamp(Float) (+ Increase%20Value (Variables|Default|GetBatteryCurrent)) 0.0 (Variables|Default|GetBatteryMax)))
  (Variables|/Game/ThirdParty/HorrorEngine/Blueprints/Player/HE_GameInstance.HE_GameInstance_C|SetCanTurnOnLights (Variables|Default|GetGameInstanceRef) true))

(event EventTick
  (params (DeltaSeconds :type Float%20%28single-precision%29))
  (bind _batteryincrement (Variables|Default|GetBatteryIncrement))
  (if (not (Variables|Default|GetbIsGameCompleted))
    (if (Variables|/Game/ThirdParty/HorrorEngine/Blueprints/Player/HE_GameInstance.HE_GameInstance_C|GetCanTurnOnLights (Variables|Default|GetGameInstanceRef))
      (if (> (Variables|Default|GetLightsVoltage) 0.0)
        (bind _output_get (Variables|Default|SetBatteryCurrent (Math|Float|Clamp(Float) (- (Variables|Default|GetBatteryCurrent) (* (Variables|Default|GetBatteryDecrement) (Variables|Default|GetLightsVoltage) DeltaSeconds (CallFunction|GetConsumptionMultiplier))) 0.0 (Variables|Default|GetBatteryMax))))
        (Variables|/Game/ThirdParty/HorrorEngine/Blueprints/Player/HE_GameInstance.HE_GameInstance_C|SetCurrentBatteryLevel (Variables|Default|GetGameInstanceRef) (Variables|Default|GetBatteryCurrent))
        (if (<= _output_get 0.5)
          (CallFunction|TriggerBlackout))
        (else
          (Variables|Default|SetBatteryCurrent (Math|Float|Clamp(Float) (+ (Variables|Default|GetBatteryCurrent) (Math|Float|SelectFloat (* _batteryincrement (Variables|Default|GetGeneratorRechargeSpeed) DeltaSeconds) _batteryincrement (Variables|Default|GetBlackoutTriggered))) 0.0 (Variables|Default|GetBatteryMax)))
          (Variables|/Game/ThirdParty/HorrorEngine/Blueprints/Player/HE_GameInstance.HE_GameInstance_C|SetCurrentBatteryLevel (Variables|Default|GetGameInstanceRef) (Variables|Default|GetBatteryCurrent))
          (if (>= (Variables|Default|GetBatteryCurrent) (Variables|Default|GetBatteryMax))
            (Variables|Default|SetBlackoutTriggered false)))))))

(event EventBeginPlay
  (bind _batterymax (Variables|Default|GetBatteryMax))
  (bind _ashe_game_instance (Utilities|Casting|CastToHE_GameInstance (Game|GetGameInstance)))
  (bind _output_get (Variables|Default|SetGameInstanceRef _ashe_game_instance))
  (Variables|/Game/ThirdParty/HorrorEngine/Blueprints/Player/HE_GameInstance.HE_GameInstance_C|SetCurrentBatteryLevel _output_get _batterymax)
  (Variables|/Game/ThirdParty/HorrorEngine/Blueprints/Player/HE_GameInstance.HE_GameInstance_C|SetCanTurnOnLights _output_get true)
  (Variables|Default|SetBatteryCurrent _batterymax)
  (Utilities|IsValid (Variables|Default|GetElectricBoxRef)
    (:Is%20Not%20Valid
      (bind _returnvalue (Actor|GetActorOfClass "/Game/ThirdParty/HousePropsFurniture/Blueprints/BP_Electricbox.BP_Electricbox_C"))
      (Variables|Default|SetElectricBoxRef _returnvalue)
      (bind _ashe_game_mode (Utilities|Casting|CastToHE_GameMode (Game|GetGameMode)))
      (EventDispatchers|BindEventtoOnGameCompleted _ashe_game_mode (delegate Custom|OnGameCompleted_Received)))))

(fn ConstructionScript)

(fn UpdateLights
  (params (LightTurnedOn :type Boolean) (LightVoltage :type Float%20%28double-precision%29))
  (bind _activelightscount (Variables|Default|GetActiveLightsCount))
  (if LightTurnedOn
    (Math|Integer|IncrementInt _activelightscount
      (:%20%20
        (Variables|Default|SetLightsVoltage (+ (Variables|Default|GetLightsVoltage) LightVoltage))
        (Variables|Default|SetBlackoutTriggered false)))
    (else
      (Math|Integer|DecrementInt _activelightscount
        (:%20%20
          (Variables|Default|SetLightsVoltage (Math|Float|Clamp(Float) (- (Variables|Default|GetLightsVoltage) LightVoltage) 0.0 1e+02))))))
  (Development|PrintString (Utilities|String|Append "Lights On:" (Utilities|String|ToString(Integer) (Variables|Default|GetActiveLightsCount)) "Voltage:" (Utilities|String|ToString(Float) (Variables|Default|GetLightsVoltage))))
  (return))

(fn TriggerBlackout
  (bind _electricboxref (Variables|Default|GetElectricBoxRef))
  (Development|PrintString "BLACKOUT!" true true "(R=1.000000,G=0.011735,B=0.000000,A=1.000000)" 4.0)
  (Variables|/Game/ThirdParty/HorrorEngine/Blueprints/Player/HE_GameInstance.HE_GameInstance_C|SetCanTurnOnLights (Variables|Default|GetGameInstanceRef) false)
  (for _array_element (Variables|Default|GetLightReferences)
    (if (Utilities|DoesObjectImplementInterface _array_element "/Game/BedtimeNightmare/Blueprints/Lights/BPI_LightInteractable.BPI_LightInteractable_C")
      (Class|BPILightInteractable|TurnOffFunction(Message) _array_element)
      (Variables|Default|SetLightsVoltage 0.0)
      (Audio|PlaySound2D "/Game/BedtimeNightmare/Audio/AC_CuttingPower_Cue.AC_CuttingPower_Cue" 0.1 1.0 0.0 0 0)
      (Variables|Default|SetBlackoutTriggered true)
      (Utilities|IsValid _electricboxref
        (:Is%20Valid
          (Default|TurnOff _electricboxref))))))

(fn GetConsumptionMultiplier
  (switch int (Variables|Default|GetActiveLightsCount)
    (:Default
      _)
    (:0
      (return 0.85))
    (:1
      (return 0.85))
    (:2
      (return 0.75))
    (:3
      (return 0.5))
    (:4
      (return 0.25))
    (:5
      _))
  (return 0.2))

(fn IncreaseBatteryMax
  (params (IncreaseAmount :type Float%20%28double-precision%29))
  (bind _output_get (Variables|Default|SetBatteryMax (+ IncreaseAmount (Variables|Default|GetBatteryMax))))
  (Variables|/Game/ThirdParty/HorrorEngine/Blueprints/Player/HE_GameInstance.HE_GameInstance_C|SetCurrentMaxBatteryLevel (Variables|Default|GetGameInstanceRef) _output_get))