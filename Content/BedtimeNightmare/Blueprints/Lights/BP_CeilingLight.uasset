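; BP_CeilingLight is a switchable ceiling point light that starts off, saving its authored intensity on BeginPlay.
; ToggleLight, gated by the game instance's CanTurnOnLights flag, switches between that intensity and zero, then reports to BP_LightManager and the linked room zone.
; TurnOff forces the light dark and directly clears the room zone's lit flag, without notifying the manager.
; GetLightIsOn exposes the current state.
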(event EventToggleLight
  (bind _roomzoneref (Variables|Default|GetRoomZoneRef))
  (if (Variables|/Game/HorrorEngine/Blueprints/Player/HE_GameInstance.HE_GameInstance_C|GetCanTurnOnLights (Variables|Default|GetGameInstanceREF))
    (bind _output_get (Variables|Default|SetIsOn (not (Variables|Default|GetIsOn))))
    (Utilities|FlowControl|Sequence
      (:then_0
        (if _output_get
          (Rendering|Components|Light|SetIntensity (Variables|Default|GetPointLight) (Variables|Default|GetMaxLightIntensity))
          (else
            (Rendering|Components|Light|SetIntensity (Variables|Default|GetPointLight) 0.0)))
        (bind _returnvalue (Actor|GetActorOfClass "/Game/BedtimeNightmare/Blueprints/Lights/BP_LightManager.BP_LightManager_C"))
        (Utilities|IsValid _returnvalue
          (:Is%20Valid
            (Default|UpdateLights _returnvalue (Variables|Default|GetIsOn) 1.0))))
      (:then_1
        (Utilities|IsValid _roomzoneref
          (:Is%20Valid
            (Default|UpdateLightStatus _roomzoneref false)))))))

(event EventBeginPlay
  (Variables|Default|SetMaxLightIntensity (Variables|/Script/Engine.LightComponentBase|GetIntensity (Variables|Default|GetPointLight)))
  (Rendering|Components|Light|SetIntensity (Variables|Default|GetPointLight) 0.0)
  (bind _ashe_game_instance (Utilities|Casting|CastToHE_GameInstance (Game|GetGameInstance)))
  (Variables|Default|SetGameInstanceREF _ashe_game_instance)
  (bind _returnvalue (Actor|GetActorOfClass "/Game/BedtimeNightmare/Blueprints/Lights/BP_LightManager.BP_LightManager_C"))
  (bind _output_get (Variables|Default|SetLightManagerRef _returnvalue)))

(fn ConstructionScript)

(fn TurnOff
  (Variables|Default|SetIsOn false)
  (Rendering|Components|Light|SetIntensity (Variables|Default|GetPointLight) 0.0)
  (Rendering|Components|Light|SetIntensity (Variables|Default|GetPointLight) 0.0)
  (Variables|/Game/BedtimeNightmare/Blueprints/Gameplay/BP_RoomZone.BP_RoomZone_C|SetIsLit (Variables|Default|GetRoomZoneRef) false))

(fn GetLightIson
  (return (Variables|Default|GetIsOn)))