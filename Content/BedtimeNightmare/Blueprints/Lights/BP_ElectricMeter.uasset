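; BP_ElectricMeter is an electric meter in Bedtime Nightmare that restores electricity when used.
; It caches a cast Game Instance on BeginPlay, and its Use event checks that instance's CanTurnOnLights flag.
; If power is off, it sets the flag and plays the switch-on sound; otherwise it plays the switch-off sound.
; Either outcome prints a status message, and the meter never clears the flag.
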(event EventBeginPlay
  (bind _ashe_game_instance (Utilities|Casting|CastTo (Game|GetGameInstance)))
  (Variables|Default|SetGameInstanceREF _ashe_game_instance))

(event EventUse
  (params (HorrorEvent :type Boolean))
  (bind _gameinstanceref (Variables|Default|GetGameInstanceREF))
  (if (Variables|Default|GetCanTurnOnLights _gameinstanceref)
    (Audio|PlaySound2D "/Game/BedtimeNightmare/Assets/Sounds/interruttore_luce_off.interruttore_luce_off" 1.0 1.0 0.0 0 0)
    (Development|PrintString "You already have electricity!")
    (else
      (Variables|Default|SetCanTurnOnLights _gameinstanceref true)
      (Audio|PlaySound2D "/Game/BedtimeNightmare/Assets/Sounds/interruttore_luce_on.interruttore_luce_on" 1.0 1.0 0.0 0 0)
      (Development|PrintString "Electricity is back! "))))

(fn ConstructionScript)