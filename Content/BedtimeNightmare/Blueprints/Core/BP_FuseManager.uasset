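; Keycard access panel, despite the FuseManager name, that opens and closes its connected electric doors.
; Use either toggles directly or prompts keycard selection from the inventory.
; Opening needs a keycard plus a disarmed alarm or admin key, otherwise showing a notice or denied feedback.
; Mesh swaps and sounds lock interaction until finished, then check horror events; construction syncs door states, and key flags persist through saves.
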(event Custom|TakeAdminKey
  ;[1 1 1] Interaction Settings
  (Variables|Default|SetAdminKey true))

(event Custom|SelectKey
  ;[1 1 1] Select Key Settings
  (bind _asmaster (CallFunction|GetPlayer))
  (bind _filteredarray (Utilities|Array|FilterArray (Variables|/Game/ThirdParty/HorrorEngine/Blueprints/Player/HorrorEngine.HorrorEngine_C|GetPlayerInventory _asmaster) "/Game/ThirdParty/HorrorEngine/Blueprints/Assets/Inventory/Keycard.Keycard_C"))
  (if (> (Utilities|Array|Length _filteredarray) 0)
    (Variables|/Game/ThirdParty/HorrorEngine/Blueprints/Player/HorrorEngine.HorrorEngine_C|SetInventoryFilter _asmaster "NewEnumerator9")
    (Variables|/Game/ThirdParty/HorrorEngine/Blueprints/Player/HorrorEngine.HorrorEngine_C|SetUseableRef _asmaster self)
    (CallFunction|SetFilteredItems "/Game/ThirdParty/HorrorEngine/Blueprints/Assets/Inventory/Keycard.Keycard_C" true true (select (Variables|KeycardControlSettings|GetOpen) "Lock" "Access"))
    (CallFunction|OpenInventory)
    (else
      (CallFunction|Notice "There is no any" "Keycard" "in inventory."))))

(event Custom|Denied
  ;[1 1 1] Denied Settings
  (Variables|Default|SetInteractionEnabled false)
  (CallFunction|SetMesh (Variables|Default|GetKeycardControl) (Variables|MeshSettings|GetDeniedMesh))
  (bind _duration (Utilities|HM3DSound 0 true (Variables|KeycardControlSettings|GetDeniedSound) (Variables|Default|GetKeycardControl) (Variables|KeycardControlSettings|GetSoundAttenuation) 0.0))
  (Utilities|FlowControl|Delay _duration)
  (CallFunction|SetMesh (Variables|Default|GetKeycardControl) (Variables|MeshSettings|GetCloseMesh))
  (Variables|Default|SetInteractionEnabled true)
  (CallFunction|HorrorEventCheck "NewEnumerator21"))

(event EventUse
  (params (HorrorEvent :type Boolean))
  ;[1 1 1] Interaction Settings
  (Utilities|HMCheckInteraction)
  (if (Variables|KeycardControlSettings|GetAskForKey)
    (if (or HorrorEvent (stale EventAlternativeUse HorrorEvent))
      (if (Variables|KeycardControlSettings|GetOpen) :!label _label
        (CallFunction|Close/Off false)
        (else
          (CallFunction|Open/On false)))
      (else
        (CallFunction|SelectKey)))
    (else
      (goto _label))))

(event EventRestoreSaveData
  (params (AssetSave :type Save%20Game%20Assets%20Structure))
  ;[0 1 0.5572] Save Settings
  (|BreakAssetSave AssetSave)
  (CallFunction|SetMesh (Variables|Default|GetKeycardControl) (select (Variables|KeycardControlSettings|GetOpen) (Variables|MeshSettings|GetOpenMesh) (Variables|MeshSettings|GetCloseMesh))))

(event EventCollectSaveData
  ;[0 1 0.5572] Save Settings
  (bind _asmaster (CallFunction|GetPlayer))
  (Utilities|Array|Add (Variables|/Game/ThirdParty/HorrorEngine/Blueprints/Core/HE_SaveGameComponent.HE_SaveGameComponent_C|GetAssetCache (Variables|/Game/ThirdParty/HorrorEngine/Blueprints/Player/HorrorEngine.HorrorEngine_C|GetHE_SaveGameComponent _asmaster)) (|MakeAssetSave)))

(event EventOpen/On
  (params (HorrorEvent :type Boolean))
  ;[1 1 1] Open / Close Settings
  (Utilities|HMCheckInteraction)
  (if (Variables|KeycardControlSettings|GetPlayerHasKey)
    (if (Variables|Default|GetDisalarmed)
      (if (not (Variables|KeycardControlSettings|GetOpen)) :!label _label
        (Variables|KeycardControlSettings|SetOpen true)
        (Default|Open/On (Variables|KeycardControlSettings|GetConnected%20E-Doors) false)
        (Utilities|FlowControl|Sequence
          (:then_0
            (Variables|Default|SetInteractionEnabled false)
            (CallFunction|SetMesh (Variables|Default|GetKeycardControl) (select (Variables|KeycardControlSettings|GetOpen) (Variables|MeshSettings|GetOpenMesh) (Variables|MeshSettings|GetCloseMesh)))
            (bind _duration (Utilities|HM3DSound 0 true (select (Variables|KeycardControlSettings|GetOpen) (Variables|KeycardControlSettings|GetCloseSound) (Variables|KeycardControlSettings|GetOpenSound)) (Variables|Default|GetKeycardControl) (Variables|KeycardControlSettings|GetSoundAttenuation) 0.0))
            (Utilities|FlowControl|Delay _duration)
            (Variables|Default|SetInteractionEnabled true)
            (CallFunction|HorrorEventCheck (select (Variables|KeycardControlSettings|GetOpen) "NewEnumerator3" "NewEnumerator4")))
          (:then_1
            (bind _asmaster (CallFunction|GetPlayer))
            (bind _filteredarray (Utilities|Array|FilterArray (Variables|/Game/ThirdParty/HorrorEngine/Blueprints/Player/HorrorEngine.HorrorEngine_C|GetPlayerInventory _asmaster) "/Game/ThirdParty/HorrorEngine/Blueprints/Assets/Inventory/Keycard.Keycard_C"))
            (for _array_element _filteredarray
              (bind _askeycard (Utilities|Casting|CastToKeycard _array_element))
              (Default|CheckUnlocked _askeycard)))))
      (elif (Variables|Default|GetAdminKey)
        (goto _label)
        (else
          (CallFunction|Denied))))
    (else
      (CallFunction|Notice "Need" "Keycard" "to access."))))

(event EventAlternativeUse
  (params (HorrorEvent :type Boolean))
  ;[1 1 1] Interaction Settings
  (Utilities|HMCheckInteraction)
  (if (Variables|KeycardControlSettings|GetAskForKey)
    (if (or (stale EventUse HorrorEvent) HorrorEvent)
      (if (Variables|KeycardControlSettings|GetOpen) :!label _label
        (CallFunction|Close/Off false)
        (else
          (CallFunction|Open/On false)))
      (else
        (CallFunction|SelectKey)))
    (else
      (goto _label))))

(event EventClose/Off
  (params (HorrorEvent :type Boolean))
  ;[1 1 1] Open / Close Settings
  (Utilities|HMCheckInteraction)
  (if HorrorEvent
    (if (Variables|KeycardControlSettings|GetOpen) :!label _label
      (Variables|KeycardControlSettings|SetOpen false)
      (Default|Close/Off (Variables|KeycardControlSettings|GetConnected%20E-Doors) false)
      (Variables|Default|SetInteractionEnabled false)
      (CallFunction|SetMesh (Variables|Default|GetKeycardControl) (select (Variables|KeycardControlSettings|GetOpen) (Variables|MeshSettings|GetOpenMesh) (Variables|MeshSettings|GetCloseMesh)))
      (bind _duration (Utilities|HM3DSound 0 true (select (Variables|KeycardControlSettings|GetOpen) (Variables|KeycardControlSettings|GetCloseSound) (Variables|KeycardControlSettings|GetOpenSound)) (Variables|Default|GetKeycardControl) (Variables|KeycardControlSettings|GetSoundAttenuation) 0.0))
      (Utilities|FlowControl|Delay _duration)
      (Variables|Default|SetInteractionEnabled true)
      (CallFunction|HorrorEventCheck (select (Variables|KeycardControlSettings|GetOpen) "NewEnumerator3" "NewEnumerator4")))
    (elif (Variables|KeycardControlSettings|GetPlayerHasKey)
      (goto _label))))

(event EventTakeKey
  (params (HorrorEvent :type Boolean))
  ;[1 1 1] Interaction Settings
  (Variables|KeycardControlSettings|SetPlayerHasKey true))

(fn ConstructionScript
  (Utilities|HMDefaultConstructions (Variables|HorrorEvents|GetCreateNewHorrorEvent))
  (if (Variables|MeshSettings|GetCloneMesh)
    (Components|InstancedStaticMesh|AddInstance (Variables|Default|GetKeycardControl) (Math|Transform|MakeTransform (Variables|MeshSettings|GetCloneMeshLocation) (Variables|MeshSettings|GetCloneMeshRotation) "1.000000,1.000000,1.000000") false))
  (Components|InstancedStaticMesh|AddInstance (Variables|Default|GetKeycardControl) (Math|Transform|MakeTransform "0, 0, 0" "0, 0, 0" "1.000000,1.000000,1.000000") false)
  (CallFunction|SetMesh (Variables|Default|GetKeycardControl) (select (Variables|KeycardControlSettings|GetOpen) (Variables|MeshSettings|GetOpenMesh) (Variables|MeshSettings|GetCloseMesh)))
  (for _array_element (Variables|KeycardControlSettings|GetConnected%20E-Doors)
    (Variables|/Game/ThirdParty/HorrorEngine/Blueprints/Assets/Interactables/Security_Door.Security_Door_C|SetOpen _array_element (Variables|KeycardControlSettings|GetOpen))
    (Default|RefreshDoor _array_element)))