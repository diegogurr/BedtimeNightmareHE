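; Spawn manager that randomly relocates a set of actors onto spawn points of matching type at level start.
; Spawn points are added through RegisterSpawnPoint; after a short BeginPlay delay, both they and the actors to relocate are shuffled.
; Each actor snap-attaches to the first point whose BPI_Spawnable type matches, prints a debug message, and removes that point from the pool.
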(event EventBeginPlay
  (bind _actorstorelocate (Variables|Default|GetActorsToRelocate))
  (Utilities|FlowControl|Delay 1.0)
  (Utilities|Array|Shuffle (Variables|Default|GetSpawnPoints))
  (Utilities|Array|Shuffle _actorstorelocate)
  (for _array_element _actorstorelocate
    (bind (_array_element_2 _array_index) (Utilities|Array|ForEachLoopwithBreak (Variables|Default|GetSpawnPoints) :!label _label)
      (:LoopBody
        (bind _aresametype (CallFunction|AreSameType _array_element (Actor|GetComponentbyClass _array_element_2 "/Game/BedtimeNightmare/Blueprints/Core/BP_SpawnPoint.BP_SpawnPoint_C")))
        (if _aresametype
          (Transformation|AttachComponentToComponent _array_element (Actor|GetComponentbyClass _array_element_2 "/Game/BedtimeNightmare/Blueprints/Core/BP_SpawnPoint.BP_SpawnPoint_C") "None" "SnapToTarget" "SnapToTarget" "KeepRelative" true)
          (Development|PrintString (Utilities|String|Append (Utilities|GetDisplayName _array_element) " in " (Utilities|GetDisplayName (Actor|GetComponentbyClass _array_element_2 "/Game/BedtimeNightmare/Blueprints/Core/BP_SpawnPoint.BP_SpawnPoint_C"))) true true "(R=0.723958,G=0.485598,B=0.000000,A=1.000000)" 5e+01)
          (Utilities|Array|RemoveIndex (Variables|Default|GetSpawnPoints) _array_index)
          (goto _label Break))))))

(fn ConstructionScript)

(fn RegisterSpawnPoint
  (params (SpawnPointRef :type Actor%20Object%20Reference))
  (Utilities|Array|Add (Variables|Default|GetSpawnPoints) SpawnPointRef))

(fn AreSameType
  (params (ObjectActor :type Actor%20Object%20Reference) (SpawnActor :type BP%20Spawn%20Point%20Object%20Reference))
  (if (and (Utilities|DoesObjectImplementInterface ObjectActor "/Game/BedtimeNightmare/Blueprints/Core/BPI_Spawnable.BPI_Spawnable_C") (Utilities|DoesObjectImplementInterface SpawnActor "/Game/BedtimeNightmare/Blueprints/Core/BPI_Spawnable.BPI_Spawnable_C"))
    (bind _spawntype (Class|BPISpawnable|GetSpawnType(Message) ObjectActor))
    (bind _spawntype_2 (Default|GetSpawnType SpawnActor))
    (return (Utilities|Enum|Equal(Enum) _spawntype_2 _spawntype))))