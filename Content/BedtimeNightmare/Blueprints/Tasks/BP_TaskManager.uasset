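; Task manager that runs the player's objective list, from randomly selected tasks through a final task to victory.
; On BeginPlay it constructs task objects, shuffles and trims them unless all are required, then binds their completion events.
; NotifyTaskFromWorld forwards pickup IDs to active tasks; completions update the GameInstance count and task list UI.
; Clearing the list adds the final task, whose completion fades out and opens the standard or Bear victory cutscene.
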(event Custom|HandleVictory
  (Input|DisableInput (Game|GetPlayerController 0))
  (bind _returnvalue (UserInterface|CreateWidget "/Game/BedtimeNightmare/Blueprints/Widget/WBP_FadeOut.WBP_FadeOut_C"))
  (UserInterface|Viewport|AddtoViewport _returnvalue 0)
  (Utilities|FlowControl|Delay 2.0)
  (Variables|/Game/ThirdParty/HorrorEngine/Blueprints/Player/HE_GameInstance.HE_GameInstance_C|GetBearEndingUnlocked (Variables|Default|GetGameInstanceREF)
    (:then
      (Game|OpenLevel(byObjectReference) "/Game/BedtimeNightmare/Maps/L_Victory_Bear_Cutscene.L_Victory_Bear_Cutscene"))
    (:else
      (Game|OpenLevel(byObjectReference) "/Game/BedtimeNightmare/Maps/L_Victory_Cutscene.L_Victory_Cutscene"))))

(event Custom|OnTaskCompleted
  (bind _tasklistuiref (Variables|Tasks|GetTaskListUIRef))
  (bind _completedtasks (Variables|Tasks|GetCompletedTasks))
  (bind _tasklistuiref_2 (Variables|Tasks|GetTaskListUIRef))
  (bind _array_element (Utilities|Array|ForEachLoopwithBreak (Variables|Tasks|GetActiveTasks) :!label _label)
    (:LoopBody
      (if (Variables|/Game/BedtimeNightmare/Blueprints/Tasks/BP_TaskBase.BP_TaskBase_C|GetIsCompleted _array_element)
        (Development|PrintString (Utilities|String|Append (Utilities|String|ToString(Name) (Variables|/Game/BedtimeNightmare/Blueprints/Tasks/BP_TaskBase.BP_TaskBase_C|GetTaskID _array_element)) " completed!"))
        (Audio|PlaySound2D "/Game/BedtimeNightmare/Audio/TaskCompleted.TaskCompleted" 0.6 1.0 0.0 0 0)
        (Default|CompleteTask _array_element)
        (Utilities|Array|RemoveItem (Variables|Tasks|GetActiveTasks) _array_element)
        (Utilities|Array|Add _completedtasks _array_element)
        (Variables|/Game/ThirdParty/HorrorEngine/Blueprints/Player/HE_GameInstance.HE_GameInstance_C|SetNumberOfTaskCompleted (Variables|Default|GetGameInstanceREF) (Utilities|Array|Length _completedtasks))
        (Utilities|IsValid _tasklistuiref
          (:Is%20Valid
            (Default|UpdateTaskList _tasklistuiref (Variables|Tasks|GetStartActiveTasks))
            (Utilities|FlowControl|Sequence
              (:then_0
                (if (== (Utilities|Array|Length (Variables|Tasks|GetActiveTasks)) 0)
                  (bind _returnvalue (Game|ConstructObjectfromClass (Variables|Tasks|GetFinalTask)))
                  (Utilities|Array|Add (Variables|Tasks|GetActiveTasks) _returnvalue)
                  (Utilities|IsValid _tasklistuiref_2
                    (:Is%20Valid
                      (Default|UpdateTaskList _tasklistuiref_2 (Variables|Tasks|GetActiveTasks))
                      (EventDispatchers|BindEventtoOnCompleted _returnvalue (delegate Custom|HandleVictory))))))
              (:then_1
                (goto _label Break)))))))))

(event EventBeginPlay
  (bind _doalltasks (Variables|TaskSettings|GetDoAllTasks))
  (bind _taskstoinitialize (Variables|Tasks|GetTasksToInitialize))
  (bind _activetasks (Variables|Tasks|GetActiveTasks))
  (bind _numberoftasks (Variables|TaskSettings|GetNumberOfTasks))
  (bind _returnvalue (Utilities|Array|Length _taskstoinitialize))
  (bind _returnvalue_2 (Math|Integer|SelectInt _returnvalue _numberoftasks _doalltasks))
  (bind _ashe_game_instance (Utilities|Casting|CastToHE_GameInstance (Game|GetGameInstance)))
  (Variables|Default|SetGameInstanceREF _ashe_game_instance)
  (for _array_element _taskstoinitialize
    (bind _returnvalue_3 (Game|ConstructObjectfromClass _array_element))
    (Utilities|IsValid _returnvalue_3
      (:Is%20Valid
        (CallFunction|AddTask _returnvalue_3))))
  (Utilities|Array|Shuffle _activetasks)
  (Utilities|Array|Resize _activetasks _returnvalue_2)
  (Variables|/Game/ThirdParty/HorrorEngine/Blueprints/Player/HE_GameInstance.HE_GameInstance_C|SetNumberOfTask (Variables|Default|GetGameInstanceREF) _returnvalue_2)
  (bind _output_get (Variables|Tasks|SetStartActiveTasks _activetasks))
  (for _array_element_2 _output_get
    (EventDispatchers|BindEventtoOnCompleted _array_element_2 (delegate Custom|OnTaskCompleted))))

(fn ConstructionScript)

(fn AddTask
  (params (Task :type BP%20Task%20Base%20Object%20Reference))
  (Utilities|Array|Add (Variables|Tasks|GetActiveTasks) Task)
  (Variables|/Game/BedtimeNightmare/Blueprints/Tasks/BP_TaskBase.BP_TaskBase_C|SetIsActive Task true))

(fn GetTaskbyID
  (params (TaskID :type Name))
  (for _array_element (Variables|Tasks|GetActiveTasks)
    (if (== (Variables|/Game/BedtimeNightmare/Blueprints/Tasks/BP_TaskBase.BP_TaskBase_C|GetTaskID _array_element) TaskID)
      _)))

(fn NotifyTaskfromWorld
  (params (IncomingID :type Name))
  (bind _array_element (Utilities|Array|ForEachLoopwithBreak (Variables|Tasks|GetActiveTasks))
    (:LoopBody
      (Default|NotifyPickup _array_element IncomingID))))