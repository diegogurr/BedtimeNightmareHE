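; BP_TaskBase is the base task for Bedtime Nightmare, tracking a pickup objective matched by TaskID.
; Matching pickups either complete it outright or, with UseCounter, raise a clamped count and broadcast progress until the target is reached.
; Drop-offs lower the count in counter mode without reverting completion.
; Completion fires OnCompleted only once, and an empty CheckIfCompleted event is left in the graph.
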(event Custom|CheckIfCompleted)

(fn CompleteTask
  (if (not (Variables|Default|GetIsCompleted))
    (Variables|Default|SetIsCompleted true)
    (Default|CallOnCompleted)))

(fn NotifyPickup
  (params (CollectedItemID :type Name))
  (if (== CollectedItemID (Variables|Default|GetTaskID))
    (if (Variables|Default|GetbUseCounter)
      (Variables|Default|SetCurrentCount (Math|Integer|Clamp(Integer) (+ (Variables|Default|GetCurrentCount) 1) 0 (Variables|Default|GetTargetCount)))
      (Default|CallOnProgressChanged)
      (if (>= (Variables|Default|GetCurrentCount) (Variables|Default|GetTargetCount))
        (CallFunction|CompleteTask))
      (else
        (CallFunction|CompleteTask)))))

(fn NotifyDropOff
  (params (CollectedItemID :type Name))
  (if (== CollectedItemID (Variables|Default|GetTaskID))
    (if (Variables|Default|GetbUseCounter)
      (Variables|Default|SetCurrentCount (Math|Integer|Clamp(Integer) (- (Variables|Default|GetCurrentCount) 1) 0 (Variables|Default|GetTargetCount)))
      (Default|CallOnProgressChanged))))