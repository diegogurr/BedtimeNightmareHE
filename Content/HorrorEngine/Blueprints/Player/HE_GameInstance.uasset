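; HE_GameInstance is a horror game instance that tracks room zones and whether any of them is lit.
; AddRoomZone and RemoveRoomZone maintain the RoomZones list, adding without duplicates and printing a debug message on each change.
; UpdateRoomLights scans the registered zones and sets PlayerInLight to true if any has IsLit set, then resets its temporary found flag.
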(fn UpdateRoomLights
  (bind _array_element (Utilities|Array|ForEachLoopwithBreak (Variables|Default|GetRoomZones))
    (:LoopBody
      (if (Variables|/Game/Blueprints/Gameplay/BP_RoomZone.BP_RoomZone_C|GetIsLit _array_element)
        (LocalVariables|SetFoundLitRoom true)))
    (:Completed
      (Variables|Default|SetPlayerInLight (LocalVariables|GetFoundLitRoom))
      (LocalVariables|SetFoundLitRoom false))))

(fn AddRoomZone
  (params (NewRoomZone :type BP%20Room%20Zone%20Object%20Reference))
  (Utilities|Array|AddUnique (Variables|Default|GetRoomZones) NewRoomZone)
  (Development|PrintString "Room Zone added"))

(fn RemoveRoomZone
  (params (RoomZoneToRemove :type BP%20Room%20Zone%20Object%20Reference))
  (Utilities|Array|RemoveItem (Variables|Default|GetRoomZones) RoomZoneToRemove)
  (Development|PrintString "Room Zone removed"))